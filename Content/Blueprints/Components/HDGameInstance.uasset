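; HDGameInstance is a game instance Blueprint that tracks player lives and runs the game-over sequence when they run out.
; LoseLife subtracts lives and fires GameOver at zero or below.
; GameOver fades the camera and hides the PuzzlePlayerCharacter's menu interface, then after a short delay shows a GameOverWidget and pauses the game.
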(event Custom|Game%20Over
  (Utilities|FlowControl|Sequence
    (:then_0
      ;[1 1 1] Fade the camera
      (CameraFades|StartCameraFade :self (Game|GetPlayerCameraManager 0) :ToAlpha 1.0 :Duration 0.25 :bHoldWhenFinished true)
      (Utilities|FlowControl|Delay 0.1)
      (bind _aspuzzle_player_character (Utilities|Casting|CastToPuzzlePlayerCharacter (Game|GetPlayerCharacter 0)))
      (Widget|SetVisibility (Variables|/Game/Blueprints/PuzzlePlayerCharacter.PuzzlePlayerCharacter_C|GetMenu%20Interface _aspuzzle_player_character) "Hidden"))
    (:then_1
      (Utilities|FlowControl|Delay 0.5)
      ;[1 1 1] Display the Gameover screen
      (bind _returnvalue (UserInterface|CreateWidget "/Game/UI/GameOverWidget.GameOverWidget_C"))
      (UserInterface|Viewport|AddtoViewport _returnvalue 0)
      (Game|SetGamePaused true))))

(fn LoseLife
  (params (LivesLost :type Integer))
  (bind _output_get (Variables|Default|SetLives (- (Variables|Default|GetLives) LivesLost)))
  (if (<= _output_get 0)
    (CallFunction|GameOver)))